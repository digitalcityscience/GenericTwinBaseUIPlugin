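; BP_WaypointIndicator is a waypoint marker for the path creator tool, with a scene capture that previews the view from that waypoint.
; Activate starts per-frame capture into a supplied render target, moves the player pawn behind and above the waypoint with matching control rotation, and shows the mesh.
; The capture excludes all waypoint indicators and the BP_PathVisualizer.
; Deactivate stops capture and hides the mesh, while SetVisibility separately toggles mesh visibility.
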(event EventBeginPlay)

(event Collision|EventActorBeginOverlap
  (params (OtherActor :type Actor%20Object%20Reference)))

(event EventTick
  (params (DeltaSeconds :type Float%20%28single-precision%29)))

(fn ConstructionScript)

(fn Activate
  (params (RenderTarget :type Texture%20Render%20Target%202D%20Object%20Reference))
  (Utilities|FlowControl|Sequence
    (:then_0
      (CallFunction|SetHiddenActors)
      (Variables|/Script/Engine.SceneCaptureComponent2D|SetTextureTarget (Variables|Default|GetSceneCapture) RenderTarget)
      (Variables|/Script/Engine.SceneCaptureComponent|SetbCaptureEveryFrame (Variables|Default|GetSceneCapture) true))
    (:then_1
      (Transformation|SetActorLocation (Game|Player|GetPlayerPawn 0) (+ (Transformation|GetActorLocation) (* (Math|Vector|GetForwardVector (Math|Rotator|MakeRotator 0.0 0.0 (.Yaw (Math|Rotator|BreakRotator (Transformation|GetActorRotation))))) -8e+02) "0.000000,0.000000,200.000000") false false)
      (Pawn|SetControlRotation (Pawn|GetController (Game|Player|GetPlayerPawn 0)) (Transformation|GetActorRotation)))
    (:then_2
      (Development|SetHiddeninGame (Variables|Default|GetMesh) false false))))

(fn Deactivate
  (Utilities|FlowControl|Sequence
    (:then_0
      (Variables|/Script/Engine.SceneCaptureComponent2D|SetTextureTarget (Variables|Default|GetSceneCapture) 0)
      (Variables|/Script/Engine.SceneCaptureComponent|SetbCaptureEveryFrame (Variables|Default|GetSceneCapture) false))
    (:then_1
      (Development|SetHiddeninGame (Variables|Default|GetMesh) true false))))

(fn SetVisibility
  (params (Visible :type Boolean))
  (Rendering|SetVisibility (Variables|Default|GetMesh) Visible false))

(fn SetHiddenActors
  (bind _outactors (Actor|GetAllActorsOfClass "BP_WaypointIndicator_C"))
  (bind _output_get (LocalVariables|SetHiddenActorsArray _outactors))
  (bind _returnvalue (Actor|GetActorOfClass "/GenericTwinBaseUIPlugin/Tools/PathCreator/PathRepresentation/BP_PathVisualizer.BP_PathVisualizer_C"))
  (Utilities|Array|Add _output_get _returnvalue)
  (Variables|/Script/Engine.SceneCaptureComponent|SetHiddenActors (Variables|Default|GetSceneCapture) (LocalVariables|GetHiddenActorsArray)))