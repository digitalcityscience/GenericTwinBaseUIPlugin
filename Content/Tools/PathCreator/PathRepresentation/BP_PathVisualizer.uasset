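; BP_PathVisualizer is a tool actor that displays an assigned path as a swept line with a sphere marker at each waypoint.
; Update rebuilds a dynamic mesh by sweeping a small circle polygon along transforms sampled from the path's spline.
; It then destroys and recreates the waypoint sphere components at each spline point, using the path's waypoint rotations.
; The line uses a dynamic material instance, and SetPathVisibility toggles the whole hierarchy.
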(event EventBeginPlay)

(event Collision|EventActorBeginOverlap
  (params (OtherActor :type Actor%20Object%20Reference)))

(event EventTick
  (params (DeltaSeconds :type Float%20%28single-precision%29)))

(fn ConstructionScript
  (bind _returnvalue (Rendering|Material|CreateDynamicMaterialInstance "/GenericTwinBaseUIPlugin/Tools/PathCreator/PathRepresentation/M_Path.M_Path" "None" "None" :!class /Script/Engine.KismetMaterialLibrary))
  (Rendering|Material|SetMaterial (Variables|Default|GetPathMesh) 0 _returnvalue)
  (Variables|Default|SetLineMaterial _returnvalue))

(fn SetPath
  (params (Path :type Generic%20Twin%20Path%20Object%20Reference))
  (Variables|Default|SetPath Path))

(fn BuildMesh
  (bind _path (Variables|Default|GetPath))
  (bind _splinecomponent (Variables|/Script/GenericTwinUtils.GenericTwinPath|GetSplineComponent _path))
  (bind _returnvalue (DynamicMeshComponent|GetDynamicMesh (Variables|Default|GetPathMesh)))
  (bind _returnvalue_2 (DynamicMesh|Reset _returnvalue))
  (if (> (Spline|GetNumberOfSplinePoints (Variables|/Script/GenericTwinUtils.GenericTwinPath|GetSplineComponent (Variables|Default|GetPath))) 1)
    (bind _returnvalue_3 (Class|GeometryScriptLibraryPolyPathFunctions|CreateCirclePath2D "(X=0.000000,Y=0.000000)" (* (Variables|Default|GetThickness) 0.5) 4))
    (bind _frames (Class|GeometryScriptLibraryPolyPathFunctions|SampleSplinetoTransforms :Spline _splinecomponent :SamplingOptions (Utilities|Struct|MakeGeometryScriptSplineSamplingOptions (* (Spline|GetNumberOfSplinePoints _splinecomponent) 20) 0.0 "UniformDistance" "Local")))
    (Class|GeometryScriptLibraryMeshPrimitiveFunctions|AppendSweepPolygon :TargetMesh _returnvalue_2 :PolygonVertices (Class|GeometryScriptLibraryPolyPathFunctions|ToArrayOfVector2D(GeometryScriptPolyPath) _returnvalue_3) :SweepPath _frames :Debug 0)))

(fn Update
  (Utilities|FlowControl|Sequence
    (:then_0
      (CallFunction|BuildMesh))
    (:then_1
      (for _array_element (Variables|Default|GetWaypoints)
        (Components|DestroyComponent _array_element))
      (Utilities|Array|Clear (Variables|Default|GetWaypoints)))
    (:then_2
      (for _index (range 0 (- (Spline|GetNumberOfSplinePoints (Variables|/Script/GenericTwinUtils.GenericTwinPath|GetSplineComponent (Variables|Default|GetPath))) 1))
        (bind _returnvalue (Game|AddComponentbyClass "/Script/Engine.StaticMeshComponent" false (Math|Transform|MakeTransform (Spline|GetLocationatSplinePoint (Variables|/Script/GenericTwinUtils.GenericTwinPath|GetSplineComponent (Variables|Default|GetPath)) _index "World") (Class|KismetMathLibrary|QuatRotator (Class|GenericTwinPath|GetRotationatWaypoint (Variables|Default|GetPath) _index)) "1.000000,1.000000,1.000000")))
        (Components|StaticMesh|SetStaticMesh _returnvalue "/Engine/BasicShapes/Sphere.Sphere")
        (Rendering|Material|SetMaterial _returnvalue 0 "/GenericTwinBaseUIPlugin/Tools/PathCreator/PathRepresentation/M_WaypointIndicator.M_WaypointIndicator")
        (Utilities|Array|Add (Variables|Default|GetWaypoints) _returnvalue)))))

(fn SetPathVisibility
  (params (Visible :type Boolean))
  (if Visible
    (Development|SetHiddeninGame (Variables|Default|GetDefaultSceneRoot) false true)
    (else
      (Development|SetHiddeninGame (Variables|Default|GetDefaultSceneRoot) true true))))